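; BP_Door_Easy is a two-panel door that moves when the player presses Interact nearby.
; TriggerBox overlaps with BP_FirstPersonCharacter enable and disable input from player controller 0, limiting interaction to that area.
; Interact plays a timeline that sets DoorMeshDown's relative location, and each update calls Play on a second timeline that moves DoorMeshUp.
; Both timelines only play forward, with no closing logic.
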(event `InputAction|Interact`
  (params (Key :type "Key Structure"))
  (:`Pressed`
    (bind (_direction _newtrack_1) (`Timeline|Timeline`)
      (:`Update`
        (`SceneComponent.K2_SetRelativeLocation` (`self.DoorMesh_Down`) _newtrack_1 false false)
        (bind (_direction_2 _newtrack_0) (`Timeline|Timeline_0`)
          (:`Update`
            (`SceneComponent.K2_SetRelativeLocation` (`self.DoorMesh_up`) _newtrack_0 false false)))))))

(event `self.TriggerBox.OnComponentBeginOverlap`
  (params (OverlappedComponent :type "PrimitiveComponent Object Reference") (OtherActor :type "Actor Object Reference") (OtherComp :type "PrimitiveComponent Object Reference") (OtherBodyIndex :type Integer) (bFromSweep :type Boolean) (SweepResult :type "HitResult Structure (by ref)"))
  (cast `/Game/Default/FirstPerson/Blueprints/BP_FirstPersonCharacter` OtherActor)
  (`self.EnableInput` (`GameplayStatics.GetPlayerController` 0)))

(event `self.TriggerBox.OnComponentEndOverlap`
  (params (OverlappedComponent :type "PrimitiveComponent Object Reference") (OtherActor :type "Actor Object Reference") (OtherComp :type "PrimitiveComponent Object Reference") (OtherBodyIndex :type Integer))
  (cast `/Game/Default/FirstPerson/Blueprints/BP_FirstPersonCharacter` OtherActor)
  (`self.DisableInput` (`GameplayStatics.GetPlayerController` 0)))

(fn `UserConstructionScript`)